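; BP_TestBuilding is a test placeable building for the build system, built around a Cube component.
; Activate and deactivate events switch the cube's collision between query-and-physics and none.
; Two preview events apply either the can-build ghost material or the can't-build material, and both also disable collision.
; Activation restores only collision, as no event here sets the material back.
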(event `self.BPActivate`
  (`PrimitiveComponent.SetCollisionEnabled` (`self.Cube`) "QueryAndPhysics"))

(event `self.BPDeActivate`
  (`PrimitiveComponent.SetCollisionEnabled` (`self.Cube`) "NoCollision"))

(event `self.SetGhostMaterial`
  (`PrimitiveComponent.SetMaterial` (`self.Cube`) 0 "/Game/buildsystem/Materials/MI_CanBuildMaterial.MI_CanBuildMaterial")
  (`PrimitiveComponent.SetCollisionEnabled` (`self.Cube`) "NoCollision" :!label _label))

(event `self.SetCantBuildMaterial`
  (`PrimitiveComponent.SetMaterial` (`self.Cube`) 0 "/Game/buildsystem/Materials/MI_CantBuildMaterial.MI_CantBuildMaterial")
  (goto _label))

(fn `UserConstructionScript`)