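; BP_Demo_1 is a placeable piece for a build system, with a cylinder mesh and a BuildingCollision component.
; Two events swap the cylinder's material to show a can-build or can't-build ghost preview, and both turn collision off.
; BPActivate and BPDeActivate switch the collision between query-and-physics and none, with no logic of its own deciding when any event fires.
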(event `self.SetGhostMaterial`
  (`PrimitiveComponent.SetMaterial` (`self.Cylinder`) 0 "/Game/buildsystem/Materials/MI_CanBuildMaterial.MI_CanBuildMaterial")
  (`PrimitiveComponent.SetCollisionEnabled` (`self.BuildingCollision`) "NoCollision"))

(event `self.SetCantBuildMaterial`
  (`PrimitiveComponent.SetMaterial` (`self.Cylinder`) 0 "/Game/buildsystem/Materials/MI_CantBuildMaterial.MI_CantBuildMaterial")
  (`PrimitiveComponent.SetCollisionEnabled` (`self.BuildingCollision`) "NoCollision"))

(event `self.BPActivate`
  (`PrimitiveComponent.SetCollisionEnabled` (`self.BuildingCollision`) "QueryAndPhysics"))

(event `self.BPDeActivate`
  (`PrimitiveComponent.SetCollisionEnabled` (`self.BuildingCollision`) "NoCollision"))

(fn `UserConstructionScript`)