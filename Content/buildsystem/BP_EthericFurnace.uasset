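; BP_EthericFurnace is a placeable crafting furnace for the build system, with placement preview states and a spinning core while crafting.
; Ghost events swap all mesh parts between can-build and can't-build materials; the latter also disables BuildingCollision, which activate and deactivate events toggle.
; Starting a craft runs a Timeline that yaws the Core and replays itself after a one-tick delay.
; Finishing only sets a flag that pins rotation to zero, so the Timeline keeps looping.
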(event `self.SetGhostMaterial`
  (`PrimitiveComponent.SetMaterial` (`self.Cylinder`) 0 "/Game/buildsystem/Materials/MI_CanBuildMaterial.MI_CanBuildMaterial")
  (`PrimitiveComponent.SetMaterial` (`self.Core`) 0 "/Game/buildsystem/Materials/MI_CanBuildMaterial.MI_CanBuildMaterial")
  (`PrimitiveComponent.SetMaterial` (`self.Cylinder_002`) 0 "/Game/buildsystem/Materials/MI_CanBuildMaterial.MI_CanBuildMaterial")
  (`PrimitiveComponent.SetMaterial` (`self.Cube_005`) 0 "/Game/buildsystem/Materials/MI_CanBuildMaterial.MI_CanBuildMaterial")
  (`PrimitiveComponent.SetMaterial` (`self.Cube_004`) 0 "/Game/buildsystem/Materials/MI_CanBuildMaterial.MI_CanBuildMaterial")
  (`PrimitiveComponent.SetMaterial` (`self.Cube_006`) 0 "/Game/buildsystem/Materials/MI_CanBuildMaterial.MI_CanBuildMaterial")
  (`PrimitiveComponent.SetMaterial` (`self.Cube_007`) 0 "/Game/buildsystem/Materials/MI_CanBuildMaterial.MI_CanBuildMaterial"))

(event `self.SetCantBuildMaterial`
  (`PrimitiveComponent.SetMaterial` (`self.Cylinder`) 0 "/Game/buildsystem/Materials/MI_CantBuildMaterial.MI_CantBuildMaterial")
  (`PrimitiveComponent.SetMaterial` (`self.Core`) 0 "/Game/buildsystem/Materials/MI_CantBuildMaterial.MI_CantBuildMaterial")
  (`PrimitiveComponent.SetMaterial` (`self.Cylinder_002`) 0 "/Game/buildsystem/Materials/MI_CantBuildMaterial.MI_CantBuildMaterial")
  (`PrimitiveComponent.SetMaterial` (`self.Cube_005`) 0 "/Game/buildsystem/Materials/MI_CantBuildMaterial.MI_CantBuildMaterial")
  (`PrimitiveComponent.SetMaterial` (`self.Cube_004`) 0 "/Game/buildsystem/Materials/MI_CantBuildMaterial.MI_CantBuildMaterial")
  (`PrimitiveComponent.SetMaterial` (`self.Cube_006`) 0 "/Game/buildsystem/Materials/MI_CantBuildMaterial.MI_CantBuildMaterial")
  (`PrimitiveComponent.SetMaterial` (`self.Cube_007`) 0 "/Game/buildsystem/Materials/MI_CantBuildMaterial.MI_CantBuildMaterial")
  (`PrimitiveComponent.SetCollisionEnabled` (`self.BuildingCollision`) "NoCollision"))

(event `self.BPActivate`
  (`PrimitiveComponent.SetCollisionEnabled` (`self.BuildingCollision`) "QueryAndPhysics"))

(event `self.BPDeActivate`
  (`PrimitiveComponent.SetCollisionEnabled` (`self.BuildingCollision`) "NoCollision"))

(event `self.BPFinishCraft`
  (set `self.isCraftFinished` true))

(event `self.BPStartCraft`
  (bind _core (`self.Core`))
  (set `self.isCraftFinished` false)
  (bind (_direction _newtrack_0) (`Timeline|Timeline` :!via `PlayFromStart` :!label _label)
    (:`Update`
      (if (`self.isCraftFinished`)
        (`SceneComponent.K2_SetRelativeRotation` _core (`KismetMathLibrary.MakeRotator` 0.0) false false)
        (else
          (`SceneComponent.K2_SetRelativeRotation` _core (`KismetMathLibrary.MakeRotator` 0.0 0.0 (`KismetMathLibrary.Lerp` 0.0 360.0 _newtrack_0)) false false))))
    (:`Finished`
      (`KismetSystemLibrary.DelayUntilNextTick`)
      (goto _label :!via `PlayFromStart`))))

(fn `UserConstructionScript`)