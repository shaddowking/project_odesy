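; BP_DemoEnemy is a demo enemy Blueprint whose graph handles only what happens when it dies.
; On the BPonDeath event it disables collision on its five cube components.
; It then casts the first player controller's HUD to BPSP_HUD and removes itself from that HUD's minimap markers.
; The construction script is empty.
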(event `self.BPOnDeath`
  (`PrimitiveComponent.SetCollisionEnabled` (`self.Cube2`) "NoCollision")
  (`PrimitiveComponent.SetCollisionEnabled` (`self.Cube1`) "NoCollision")
  (`PrimitiveComponent.SetCollisionEnabled` (`self.Cube`) "NoCollision")
  (`PrimitiveComponent.SetCollisionEnabled` (`self.Cube4`) "NoCollision")
  (`PrimitiveComponent.SetCollisionEnabled` (`self.Cube3`) "NoCollision")
  (bind _asbpsp_hud (cast `/Game/BPSP_HUD` (`PlayerController.GetHUD` (`GameplayStatics.GetPlayerController` 0))))
  (`Minimap.RemoveMarker` (`SP_HUD.Minimap` _asbpsp_hud) self))

(fn `UserConstructionScript`)