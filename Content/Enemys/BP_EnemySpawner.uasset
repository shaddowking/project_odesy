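; BP_EnemySpawner is an enemy spawner actor that registers itself with the game instance's ExploreManager one tick after BeginPlay.
; DeactivateSpawner teleports every enemy in CreatedEnemys to the BP_EnemyHolder actor's location instead of destroying them.
; The construction script fits a box visual to the spawn range and height.
; A delayed, data-list-driven spawn loop exists in the event graph but is disconnected and never runs.
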(event `self.ReceiveBeginPlay`
  (`KismetSystemLibrary.DelayUntilNextTick`)
  (bind _asgi_spgame_istance (cast `/Game/GI_SPGameIstance` (`GameplayStatics.GetGameInstance`)))
  (`KismetArrayLibrary.Array_Add` (`ExploreManager.EnemySpawnerList` (`SPGameInstance.ExploreManager` _asgi_spgame_istance)) self))

(event `self.DeactivateSpawner`
  (bind _returnvalue (`GameplayStatics.GetActorOfClass` "/Game/Enemys/BP_EnemyHolder.BP_EnemyHolder_C"))
  (for _array_element (`self.CreatedEnemys`)
    (`self.K2_SetActorLocation` _array_element (`self.K2_GetActorLocation` _returnvalue) false true)))

(fn `UserConstructionScript`
  (bind _spawnrange (`self.SpawnRange`))
  (`BoxComponent.SetBoxExtent` (`self.SpawnRangeVisual`) (`KismetMathLibrary.MakeVector` _spawnrange _spawnrange 32.0) true)
  (`SceneComponent.K2_SetRelativeLocation` (`self.SpawnRangeVisual`) (`KismetMathLibrary.MakeVector` 0.0 0.0 (`self.SpawnHight`)) false false))