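; Storm turret actor for the Stormwalker's Storm's Eye ability, providing the turret's lightning activation visual.
; On BeginPlay it creates a dynamic M_Core material instance, stores it and applies it to the Sphere, though nothing here animates it.
; BPActivate points the Niagara lightning beam's end at the Sphere's world location, then flashes the beam briefly using a Delay before deactivating it.
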(event `self.ReceiveBeginPlay`
  (bind _returnvalue (`KismetMaterialLibrary.CreateDynamicMaterialInstance` "/Game/Abilitys/Stormwalker/StormsEye/M_Core.M_Core"))
  (bind _output_get (set `self.core materal` _returnvalue))
  (`PrimitiveComponent.SetMaterial` (`self.Sphere`) 0 _output_get))

(event `self.BPActivate`
  (params (Location :type "Vector Structure"))
  (bind _ns_lightningbeam (`self.NS_LightningBeam`))
  (`NiagaraComponent.SetNiagaraVariableVec3` _ns_lightningbeam "Beam End" (`SceneComponent.K2_GetComponentLocation` (`self.Sphere`)))
  (`ActorComponent.Activate` _ns_lightningbeam true)
  (`KismetSystemLibrary.Delay` 0.2)
  (`ActorComponent.Deactivate` _ns_lightningbeam))

(fn `UserConstructionScript`)