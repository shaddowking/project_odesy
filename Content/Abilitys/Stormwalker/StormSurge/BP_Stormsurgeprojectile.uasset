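; Projectile actor for the Stormwalker's Storm Surge ability that flashes lightning beams toward given locations.
; BeginPlay pre-creates a pool of deactivated lightning beam Niagara components in LightningList.
; StartLightningVFX takes the first inactive beam, sets its end to the target location, then after a brief delay deactivates it and resets the end to the actor.
; When every beam is busy, GetNextLaser reuses the one at index 1.
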(event `self.ReceiveBeginPlay`
  (for _ (range (+ (`self.laserCount`) 1))
    (bind _returnvalue (`AddComponent|NODE_AddNiagaraComponent-1`))
    (`NiagaraComponent.SetAsset` _returnvalue "/Game/VFX/NS_LightningBeam.NS_LightningBeam" true)
    (`ActorComponent.SetAutoActivate` _returnvalue false)
    (`ActorComponent.Deactivate` _returnvalue)
    (`KismetArrayLibrary.Array_Add` (`self.LightningList`) _returnvalue)))

(event `self.StartLightningVFX`
  (params (Location :type "Vector Structure"))
  (bind _newparam (`self.GetNextLaser`))
  (`ActorComponent.Activate` _newparam true)
  (`NiagaraComponent.SetNiagaraVariableVec3` _newparam "Beam End" Location)
  (`KismetSystemLibrary.Delay` 0.1)
  (`ActorComponent.Deactivate` _newparam)
  (`NiagaraComponent.SetNiagaraVariableVec3` _newparam "Beam End" (`self.K2_GetActorLocation`)))

(fn `GetNextLaser`
  (returns (NewParam :type "NiagaraComponent Object Reference"))
  (bind _lightninglist (`self.LightningList`))
  (for _array_element _lightninglist
    (if (not (`ActorComponent.IsActive` _array_element))
      (return _array_element)))
  (return (`|GetArrayItem` _lightninglist 1)))

(fn `UserConstructionScript`)