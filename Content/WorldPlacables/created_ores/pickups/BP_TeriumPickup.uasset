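; BP_TeriumPickup is a Terium ore pickup actor with a widget that turns to face the player.
; Each Tick yaws the widget toward player 0's viewpoint, keeping its existing pitch and roll.
; The BPActivet and BPDeactivet events switch actor tick on and off, so the facing update runs only while tick is enabled.
; This graph holds no overlap or collection logic.
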(event `self.ReceiveBeginPlay`)

(event `self.ReceiveTick`
  (params (DeltaSeconds :type "Float (single-precision)"))
  (bind _widget (`self.Widget`))
  (bind (_returnvalue_roll _returnvalue_pitch) (`KismetMathLibrary.BreakRotator` (`SceneComponent.K2_GetComponentRotation` _widget)))
  (bind (_returnvalue_roll_2 _returnvalue_pitch_2 _returnvalue_yaw) (`KismetMathLibrary.BreakRotator` (`KismetMathLibrary.FindLookAtRotation` (`self.K2_GetActorLocation`) (`Controller.GetPlayerViewPoint` (`GameplayStatics.GetPlayerController` 0)))))
  (`SceneComponent.K2_SetWorldRotation` _widget (`KismetMathLibrary.MakeRotator` _returnvalue_roll _returnvalue_pitch _returnvalue_yaw) false false))

(event `self.BPActivet`
  (`self.SetActorTickEnabled` true))

(event `self.BPDeactivet`
  (`self.SetActorTickEnabled` false))

(fn `UserConstructionScript`)